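; Rope attach point actor that shows a DetectionNode widget marking where the player can hook.
; BeginPlay caches the widget; each Tick, while in focus, sizes its white fill from a clamped player-distance value, turning green at full size and hiding it when small or unfocused.
; Using the point plays a fast PopOut animation, pausing UI updates for roughly ten frames.
; SetActive toggles the active flag and visibility; ChangeState is an empty event.
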(event `self.ReceiveBeginPlay`
  (bind _asdetection_node (cast `/Game/Rope/Widgets/DetectionNode` (`WidgetComponent.GetUserWidgetObject` (`self.Widget`))))
  (set `self.WidgetReference` _asdetection_node))

(event `self.ReceiveTick`
  (params (DeltaSeconds :type "Float (single-precision)"))
  (`self.Show UIPlayer Distance`))

(event `self.PlayAnimationOnUse`
  (bind _widgetreference (`self.WidgetReference`))
  (set `self.bUpdatingUI` false)
  (`UserWidget.PlayAnimation` _widgetreference (`/Game/Rope/Widgets/DetectionNode.PopOut` _widgetreference) 0.0 1 "Forward" 5.0 true)
  (`KismetSystemLibrary.Delay` (* (`GameplayStatics.GetWorldDeltaSeconds`) 10.0))
  (set `self.bUpdatingUI` true))

(event `self.ChangeState`
  (params (AttachPointState :type "EAttachPointState Enum" :default "OutRangeState")))

(fn `SetActive`
  (params (Condition :type Boolean))
  (bind _widgetreference (`self.WidgetReference`))
  (if Condition
    (set `self.bActive` true)
    (`Widget.SetVisibility` _widgetreference "Visible")
    (else
      (set `self.bActive` false)
      (`Widget.SetVisibility` _widgetreference "Hidden"))))

(fn `Show UIPlayer Distance`
  (bind _widgetreference (`self.WidgetReference`))
  (bind _distancedfromplayerclamped (`self.DistancedFromPlayerClamped`))
  (bind _widgetreference_2 (`self.WidgetReference`))
  (bind _whitefilled (`/Game/Rope/Widgets/DetectionNode.WhiteFilled` (`self.WidgetReference`)))
  ;[1 1 1] Show UI When Player is close Enough
  (if (`self.bUpdatingUI`)
    (if (`|EnumEquality` (`self.AttachPointState`) "InFocusState")
      (`Widget.SetVisibility` _widgetreference_2 "Visible")
      (`Image.SetBrushSize` _whitefilled (`KismetMathLibrary.MakeVector2D` _distancedfromplayerclamped _distancedfromplayerclamped))
      (`Image.SetColorAndOpacity` _whitefilled (select `bool` (== _distancedfromplayerclamped 100.0) :`false` (struct :`R` 1.0 :`G` 1.0 :`B` 1.0 :`A` 1.0) :`true` (struct :`R` 0.1841 :`G` 0.630208 :`B` 0.206321 :`A` 1.0) :!type "LinearColor Structure"))
      (if (or (< _distancedfromplayerclamped 20.0) false)
        (`Widget.SetVisibility` _widgetreference "Hidden")
        (else
          (`Widget.SetVisibility` _widgetreference "Visible")))
      (else
        (`Widget.SetVisibility` _widgetreference_2 "Hidden")))))

(fn `UserConstructionScript`)