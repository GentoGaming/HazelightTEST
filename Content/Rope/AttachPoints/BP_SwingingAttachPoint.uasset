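; Rope swing attach point that shows a DetectionNode widget indicating the player's proximity and the point's state.
; On BeginPlay it caches the widget, then every Tick resizes its fill from a clamped player distance value, turning green at maximum and hiding at low values.
; State changes show the widget when in focus, play a pop-out before hiding when in use, and hide it otherwise.
; SetActive toggles the active flag and widget visibility together.
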(event `self.ReceiveBeginPlay`
  ;[1 1 1] UI Update , Enable Disable Tick Based on Player Location .
  (bind _asdetection_node (cast `/Game/Rope/Widgets/DetectionNode` (`WidgetComponent.GetUserWidgetObject` (`self.Widget`))))
  (set `self.WidgetReference` _asdetection_node))

(event `self.ReceiveTick`
  (params (DeltaSeconds :type "Float (single-precision)"))
  (bind _widgetreference (`self.WidgetReference`))
  (bind _distancedfromplayerclamped (`self.DistancedFromPlayerClamped`))
  (bind _whitefilled (`/Game/Rope/Widgets/DetectionNode.WhiteFilled` (`self.WidgetReference`)))
  ;[1 1 1] UI Update , Enable Disable Tick Based on Player Location .
  (`Image.SetBrushSize` _whitefilled (`KismetMathLibrary.MakeVector2D` _distancedfromplayerclamped _distancedfromplayerclamped))
  (`Image.SetColorAndOpacity` _whitefilled (select `bool` (== _distancedfromplayerclamped 100.0) :`false` (struct :`R` 1.0 :`G` 1.0 :`B` 1.0 :`A` 1.0) :`true` (struct :`R` 0.1841 :`G` 0.630208 :`B` 0.206321 :`A` 1.0) :!type "LinearColor Structure"))
  (if (or (< _distancedfromplayerclamped 20.0) false)
    (`Widget.SetVisibility` _widgetreference "Hidden")
    (else
      (`Widget.SetVisibility` _widgetreference "Visible"))))

(event `self.ChangeAttachPointState`
  (params (State :type "EAttachPointState Enum" :default "OutRangeState"))
  (bind _widgetreference (`self.WidgetReference`))
  (bind _widgetreference_2 (`self.WidgetReference`))
  ;[1 1 1] UI Update , Enable Disable Tick Based on Player Location .
  (switch `EAttachPointState` State
    (:`OutRangeState`
      (`Widget.SetVisibility` _widgetreference_2 "Hidden" :!label _label))
    (:`InRangeState`
      (goto _label))
    (:`InFocusState`
      (`Widget.SetVisibility` _widgetreference_2 "Visible"))
    (:`InUseState`
      (`UserWidget.PlayAnimation` _widgetreference (`/Game/Rope/Widgets/DetectionNode.PopOut` _widgetreference) 0.0 1 "Forward" 3.0 false)
      (`KismetSystemLibrary.Delay` 0.3)
      (goto _label))
    (:`InBlockViewState`
      (goto _label))))

(fn `SetActive`
  (params (Condition :type Boolean))
  (bind _widgetreference (`self.WidgetReference`))
  (if Condition
    (set `self.bActive` true)
    (`Widget.SetVisibility` _widgetreference "Visible")
    (else
      (set `self.bActive` false)
      (`Widget.SetVisibility` _widgetreference "Hidden"))))

(fn `Show UIPlayer Distance`
  ;[1 1 1] Show UI When Player is close Enough
)

(fn `UserConstructionScript`)